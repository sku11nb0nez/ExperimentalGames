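; Player frog character with a charged, mouse-aimed jump locked to the Y-Z plane.
; Holding IA_Jump builds charge each Tick to scale launch strength, aiming at the cursor hit point; releasing calls LaunchCharacter.
; DrawJumpPrediction previews the arc with gravity-based projectile math and debug lines.
; It also creates the HUD and opens its pause screen on P; tongue input is an unimplemented stub.
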(event `EnhancedInput|/Game/frog/InputAction/IA_Tongue`
  (params (ActionValue :type Boolean) (ElapsedSeconds :type "Float (double-precision)") (TriggeredSeconds :type "Float (double-precision)") (InputAction :type "InputAction Object Reference" :default "/Game/frog/InputAction/IA_Tongue.IA_Tongue")))

(event `self.ReceiveTick`
  (params (DeltaSeconds :type "Float (single-precision)"))
  ; Continually checks if Jump has been triggered
  (if (`self.IsChargingJump`)
    ; Calculate the length of time jump has been held + max charge amount * secs -> clamp value so its no more than the max jump amount allowed
    (set `self.JumpChargeAmount` (`KismetMathLibrary.FClamp` (+ (`self.JumpChargeAmount`) (* (`self.JumpChargeMax`) DeltaSeconds)) 0.0 (`self.JumpChargeMax`)))
    ; Divide the charge amount by the max to get a % set that as charge percent - lerp node finds the Jump strength by calculating where the strength falls by through the percentage
    (bind _output_get (set `self.Charge Percent` (/ (`self.JumpChargeAmount`) (`self.JumpChargeMax`))))
    (set `self.Jumpstrength` (`KismetMathLibrary.Lerp` (`self.MinJumpStrength`) (`self.MaxJumpStrenght`) _output_get))
    ; Jump Direction + strength are multiplied to predict the velocity of the jump and a prediction line in developed based on this
    (bind _output_get_2 (set `self.JumpDirection` (`KismetMathLibrary.Normal` (`KismetMathLibrary.MakeVector` 0.0 (.y (- (`.ImpactPoint` (`GameplayStatics.BreakHitResult` (`PlayerController.GetHitResultUnderCursorByChannel` (`GameplayStatics.GetPlayerController` 0) "TraceTypeQuery2" true))) (`self.K2_GetActorLocation`))) (.z (- (`.ImpactPoint` (`GameplayStatics.BreakHitResult` (`PlayerController.GetHitResultUnderCursorByChannel` (`GameplayStatics.GetPlayerController` 0) "TraceTypeQuery2" true))) (`self.K2_GetActorLocation`)))))))
    (bind _output_get_3 (set `self.PreviewVelocity` (* _output_get_2 (`self.Jumpstrength`))))
    (`self.DrawJumpPrediction` (`self.K2_GetActorLocation`) _output_get_3)))

(event `EnhancedInput|/Game/Input/Actions/IA_Jump`
  (params (ActionValue :type Boolean) (ElapsedSeconds :type "Float (double-precision)") (TriggeredSeconds :type "Float (double-precision)") (InputAction :type "InputAction Object Reference" :default "/Game/Input/Actions/IA_Jump.IA_Jump"))
  (:`Started`
    ; If player starts holding the jump button reset amount to 0
    (set `self.IsChargingJump` true)
    (set `self.JumpChargeAmount` 0.0))
  (:`Completed`
    ; If the player is jumping
    (if (`self.IsChargingJump`)
      ; Use the result from the multiplication as the launch velocity and what direction the character should be launched in - Set charging jump back to false when completed
      (`self.LaunchCharacter` (* (`self.JumpDirection`) (`KismetMathLibrary.Lerp` (`self.MinJumpStrength`) (`self.MaxJumpStrenght`) (/ (`self.JumpChargeAmount`) (`self.JumpChargeMax`)))))
      (set `self.IsChargingJump` false))))

(event `self.ReceiveBeginPlay`
  (`EnhancedInputSubsystemInterface.AddMappingContext` (pcsubsystem `EnhancedInputLocalPlayerSubsystem` (`GameplayStatics.GetPlayerController` 0)) "/Game/frog/InputAction/IMC_Frog.IMC_Frog" 0 (struct))
  (set `PlayerController.bShowMouseCursor` true (`GameplayStatics.GetPlayerController` 0))
  ; Adding HUD to Viewport
  (bind _returnvalue (`|CreateWidget` "/Game/UI/WB_HUD.WB_HUD_C"))
  (bind _output_get (set `self.HUD` _returnvalue))
  (`UserWidget.AddToViewport` _output_get 0))

(event `Key|P`
  (params (Key :type "Key Structure"))
  (bind _returnvalue (`GameplayStatics.GetPlayerController` 0))
  ; HUD
  ;; Pause Menu Button
  (:`Pressed`
    (`GameplayStatics.PlaySound2D` "/Game/UI/SoundFX/wav__HD_/JDSherbert_-_Ultimate_UI_SFX_Pack_-_Popup_Open_-_1.JDSherbert_-_Ultimate_UI_SFX_Pack_-_Popup_Open_-_1" 1.0 1.0 0.0 null null)
    (set `Widget.Visibility` "Visible" (`/Game/UI/WB_HUD.Pause_Screen` (`self.HUD`)))
    (set `PlayerController.bShowMouseCursor` true _returnvalue)
    (`GameplayStatics.SetGamePaused` true)
    (`WidgetBlueprintLibrary.SetInputMode_UIOnlyEx` _returnvalue null)))

(fn `DrawJumpPrediction`
  (params (StartLocation :type "Vector Structure") (LaunchVelocity :type "Vector Structure"))
  (locals (PreviousPoint :type "Vector Structure") (Time :type "Float (double-precision)") (`Gravity Displacement` :type "Float (double-precision)") (`Gravity vector` :type "Vector Structure" :default (0.0 0.0 0.0)) (Currentpoint :type "Vector Structure"))
  (set `local.PreviousPoint` StartLocation)
  (for _index (range 21)
    (set `local.Time` (* _index 0.05))
    (bind _output_get (set `local.Gravity Displacement` (* (* (`MovementComponent.GetGravityZ` (`self.CharacterMovement`)) (* (`local.Time`) (`local.Time`))) 0.5)))
    (bind _output_get_2 (set `local.Gravity vector` (`KismetMathLibrary.MakeVector` 0.0 0.0 _output_get)))
    (set `local.Currentpoint` (+ _output_get_2 (+ (* LaunchVelocity (`local.Time`)) StartLocation)))
    (`KismetSystemLibrary.DrawDebugLine` (`local.PreviousPoint`) (`local.Currentpoint`) (struct :`R` 1.0 :`G` 1.0 :`B` 1.0 :`A` 1.0) 0.0 5.0)
    (set `local.PreviousPoint` (`local.Currentpoint`))))

(fn `UserConstructionScript`)