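; BP_FrogTongue is an actor that draws a frog's tongue as a spline mesh with variable direction and length.
; Its UpdateTongue event rebuilds a two-point spline along local Y, aims the mesh's Y axis at Direction, copies points and tangents to it, then moves the actor to StartLocation.
; The first point takes the spline's world location as a local position, and an actor-rotation node is left unconnected.
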(event `UpdateTongue`
  (params (Direction :type "Vector Structure") (Length :type "Float (double-precision)") (StartLocation :type "Vector Structure"))
  (bind _spline (`self.Spline`))
  (bind _spline_2 (`self.Spline`))
  (`SplineComponent.ClearSplinePoints` (`self.Spline`) true)
  (`SceneComponent.K2_SetWorldRotation` (`self.SplineMesh`) (`KismetMathLibrary.MakeRotFromY` Direction) false false)
  (`SplineComponent.AddSplinePointAtIndex` _spline (`SceneComponent.K2_GetComponentLocation` _spline) 0 "Local" true)
  (`SplineComponent.AddSplinePointAtIndex` _spline (`KismetMathLibrary.MakeVector` 0.0 Length) 1 "Local" true)
  (`SplineMeshComponent.SetStartAndEnd` (`self.SplineMesh`) (`SplineComponent.GetLocationAtSplinePoint` _spline_2 0 "Local") (`SplineComponent.GetTangentAtSplinePoint` _spline_2 0 "Local") (`SplineComponent.GetLocationAtSplinePoint` _spline_2 1 "Local") (`SplineComponent.GetTangentAtSplinePoint` _spline_2 1 "Local") true)
  (`self.K2_SetActorLocation` StartLocation))

(fn `UserConstructionScript`)